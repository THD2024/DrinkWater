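; BP_NewContainer is an interactable container item with two doors that swing open and closed.
; OwnInteractAnim plays a 2D interact sound, then uses a FlipFlop to alternate the OpenDoor timeline between forward and reverse.
; The timeline rotates the left and right pivots in opposite yaw directions and passes its alpha to the sound as a float parameter.
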(event EventBeginPlay)

(event Collision|EventActorBeginOverlap
  (params (OtherActor :type Actor%20Object%20Reference)))

(event EventTick
  (params (DeltaSeconds :type Float%20%28single-precision%29)))

(event EventOwnInteractAnim
  (Audio|PlaySound2D (Variables|Default|GetItemInteractSound) 1.0 1.0 0.0 0 0)
  (Utilities|FlowControl|FlipFlop
    (:A
      (bind _dooropen (Timeline|OpenDoor PlayFromStart)
        (:Update
          (Transformation|SetRelativeRotation (Variables|Default|GetR_Pivot) (Math|Rotator|Lerp(Rotator) (Math|Rotator|MakeRotator 0.0 0.0 0.0) (Math|Rotator|MakeRotator 0.0 0.0 -9e+01) _dooropen) false false)
          (Transformation|SetRelativeRotation (Variables|Default|GetL_Pivot) (Math|Rotator|Lerp(Rotator) (Math|Rotator|MakeRotator 0.0 0.0 0.0) (Math|Rotator|MakeRotator 0.0 0.0 9e+01) _dooropen) false false)
          (Audio|Parameter|SetFloatParameter (Variables|Default|GetItemInteractSound) "TimeLineAlpha" _dooropen :!class /Script/AudioExtensions.AudioParameterControllerInterface))))
    (:B
      (Timeline|OpenDoor ReverseFromEnd))))

(fn ConstructionScript)